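; BP_BrueckenRaetzel is a bridge puzzle trigger that gates the end sequence on whether the player has the wood item.
; On overlap it checks HasWoodDings on the first-person character, then either has BPSequencer play the end sequence or shows TextLins through the player's MainUI.
; The character reference is cached after the first successful cast, so later overlaps by any actor skip the cast and test that player.
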(event `self.ReceiveActorBeginOverlap`
  (params (OtherActor :type "Actor Object Reference"))
  (`/Engine/EditorBlueprintResources/StandardMacros.IsValid` (`self.First Persion Character`)
    (:`Is Valid`
      _)
    (:`Is Not Valid`
      (bind _asbp_first_persion_character (cast `/Game/Blueprints/Player/BP_FirstPersionCharacter` OtherActor))
      (bind _output_get (set `self.First Persion Character` _asbp_first_persion_character))))
  (if (`/Game/Blueprints/Player/BP_FirstPersionCharacter.HasWoodDings` _output_get)
    (`/Game/Sequence/BP_Sequence.SequenceEvent_PlayEndSequence` (`self.BP_Sequencer`) false false)
    (else
      (`/Game/Blueprints/UI/BPW_MainUI.UIEvent_ShowText` (`/Game/Blueprints/Player/BP_FirstPersionCharacter.MainUI` _output_get) (`self.Text Lins`) true 2.0))))

(fn `UserConstructionScript`)