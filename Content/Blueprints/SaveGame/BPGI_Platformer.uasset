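; Game instance for the platformer that owns the persistent settings save and applies saved audio volumes at startup.
; On Init it loads or creates the Settings save object, then retries each tick until a GameMode is valid.
; It then pushes a sound mix with Master, music and SFX class volume overrides.
; Shutdown writes the save to its slot, and a getter exposes it to other Blueprints.
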(event `self.ReceiveInit`
  (bind _returnvalue (`GameplayStatics.DoesSaveGameExist` "Settings"))
  (if _returnvalue
    (bind _returnvalue_2 (`GameplayStatics.LoadGameFromSlot` "Settings"))
    (bind _asbp_settings_save (cast `/Game/Blueprints/SaveGame/BP_SettingsSave` _returnvalue_2))
    (set `self.Settings Save` _asbp_settings_save)
    (else
      (bind _returnvalue_3 (`GameplayStatics.CreateSaveGameObject` "/Game/Blueprints/SaveGame/BP_SettingsSave.BP_SettingsSave_C"))
      (set `self.Settings Save` _returnvalue_3)))
  (`/Engine/EditorBlueprintResources/StandardMacros.IsValid` (`GameplayStatics.GetGameMode`) :!label _label
    (:`Is Valid`
      (`GameplayStatics.SetSoundMixClassOverride` "/Game/Sounds/HRK_SoundMix.HRK_SoundMix" "/Game/Sounds/HTK_Master.HTK_Master" (`/Game/Blueprints/SaveGame/BP_SettingsSave.MasterVolium` (`self.Settings Save`)))
      (`GameplayStatics.SetSoundMixClassOverride` "/Game/Sounds/HRK_SoundMix.HRK_SoundMix" "/Game/Sounds/HTK_Musik.HTK_Musik" (`/Game/Blueprints/SaveGame/BP_SettingsSave.MusikVolium` (`self.Settings Save`)))
      (`GameplayStatics.SetSoundMixClassOverride` "/Game/Sounds/HRK_SoundMix.HRK_SoundMix" "/Game/Sounds/HTK_SFX.HTK_SFX" (`/Game/Blueprints/SaveGame/BP_SettingsSave.SFXVolium` (`self.Settings Save`)))
      (`GameplayStatics.PushSoundMixModifier` "/Game/Sounds/HRK_SoundMix.HRK_SoundMix"))
    (:`Is Not Valid`
      (`KismetSystemLibrary.DelayUntilNextTick`)
      (goto _label))))

(event `self.ReceiveShutdown`
  (`GameplayStatics.SaveGameToSlot` (`self.Settings Save`) "Settings"))

(fn `ReturnSettingsSave`
  (params (test :type Boolean))
  (returns (SettingaSave :type "/Game/Blueprints/SaveGame/BP_SettingsSave Object Reference"))
  (return (`self.Settings Save`)))