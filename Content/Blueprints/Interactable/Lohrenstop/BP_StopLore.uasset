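; BP_StopLore is an interactable stop trigger that blocks forward spline movement of a BP_Lore actor while it overlaps.
; The first BP_Lore to enter is cached, and only that actor triggers the stop afterwards.
; Entering sets its forward-stop flag, calls its stop functions and shows TextLins through the player's main UI.
; Leaving only clears the flag, and player interaction does nothing.
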(event `self.ReceiveActorEndOverlap`
  (params (OtherActor :type "Actor Object Reference"))
  (`parent.ReceiveActorEndOverlap` OtherActor)
  (if (== OtherActor (`self.As BP Lore`))
    ; SteinBlock
    (set `/Game/Blueprints/Lore/BP_Lore.StopLohreSpline_1_Forward` false (`self.As BP Lore`))))

(event `self.ReceiveActorBeginOverlap`
  (params (OtherActor :type "Actor Object Reference"))
  (`parent.ReceiveActorBeginOverlap` OtherActor)
  (`/Engine/EditorBlueprintResources/StandardMacros.IsValid` (`self.As BP Lore`)
    (:`Is Valid`
      (if (== (`self.As BP Lore`) OtherActor)
        ; SteinBlock
        (set `/Game/Blueprints/Lore/BP_Lore.StopLohreSpline_1_Forward` true (stale _output_get) :!label _label)
        (`/Game/Blueprints/Lore/BP_Lore.StopLoreAnimation_1` (stale _output_get))
        (`/Game/Blueprints/Lore/BP_Lore.StopTotoLore` (stale _output_get))
        (`/Game/Blueprints/UI/BPW_MainUI.UIEvent_ShowText` (`/Game/Blueprints/Player/BP_FirstPersionCharacter.MainUI` (`/Game/Blueprints/BP_ParentControllableInteractable.Player` (stale _output_get))) (`self.Text Lins`) true 2.0)))
    (:`Is Not Valid`
      (bind _asbp_lore (cast `/Game/Blueprints/Lore/BP_Lore` OtherActor))
      (bind _output_get (set `self.As BP Lore` _asbp_lore))
      (goto _label))))

(event `self.PlayerInteract`)

(fn `UserConstructionScript`
  (`parent.UserConstructionScript`))