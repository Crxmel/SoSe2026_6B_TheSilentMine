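; Interactable stone that a player carrying a pickaxe can clear, built as a child Blueprint of a parent interactable.
; On interaction it enables physics on the stone mesh and launches it upward with an impulse.
; After a short delay, a timeline rescales the mesh by multiplying its current world scale by the curve value each update, then destroys the actor when finished.
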(event `self.PlayerInteract`
  (bind _gc_stone_no_2_low (`self.GC_Stone_NO_2_low`))
  (if (`/Game/Blueprints/Player/BP_FirstPersionCharacter.HasPickaxe` (`self.Player`))
    (`PrimitiveComponent.SetSimulatePhysics` _gc_stone_no_2_low true)
    (`PrimitiveComponent.AddImpulse` _gc_stone_no_2_low (0.0 0.0 3000.0) "None" false)
    (`KismetSystemLibrary.Delay` 1.0)
    (bind (_direction _newtrack_0) (`Timeline|Timeline` :!via `PlayFromStart`)
      (:`Update`
        (`SceneComponent.SetRelativeScale3D` _gc_stone_no_2_low (* _newtrack_0 (`SceneComponent.K2_GetComponentScale` _gc_stone_no_2_low))))
      (:`Finished`
        (`self.K2_DestroyActor`)))))

(fn `UserConstructionScript`
  (`parent.UserConstructionScript`))