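; Interactable lever that starts the upper and lower elevator animations once the player and a weighted Lore are on the elevator.
; On interact it passes itself to both elevators, waits a frame, then checks its condition flags.
; Success plays the sound and pull timeline once, then animates both elevators; failure shows context-specific UI text.
; A Debug flag bypasses the checks and is cleared in distribution builds.
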(event `self.PlayerInteract`
  (if (`self.Debug`)
    (`AudioComponent.Play` (`self.SC_InteractLever`) 0.0 :!label _label)
    ; Animation
    (bind (_direction _rotate) (`Timeline|Timeline`)
      (:`Update`
        (`SceneComponent.K2_SetRelativeRotation` (`self.Scene`) (`KismetMathLibrary.MakeRotator` 0.0 (* _rotate 50.0)) false false))
      (:`Finished`
        (`/Game/Blueprints/BP_ElevatorParent.PlayAnimation` (`self.ElevatorDown`))
        (`/Game/Blueprints/BP_ElevatorParent.PlayAnimation` (`self.ElevatorUp`))))
    (else
      (`/Game/Blueprints/BP_ElevatorParent.InteractWithLever` (`self.ElevatorDown`) self)
      (`/Game/Blueprints/BP_ElevatorParent.InteractWithLever` (`self.ElevatorUp`) self)
      (`KismetSystemLibrary.DelayUntilNextFrame`)
      (if (and (`self.LoreOnElevatorAndHasWight`) (`self.PlayerOnElevator`))
        (`/Engine/EditorBlueprintResources/StandardMacros.DoOnce` false
          (:`Completed`
            (goto _label)))
        (else
          ; Text
          (if (`self.PlayerOnElevator`)
            (if (`self.LoreOnElevatorAnd_DONT_HasWight`)
              (`/Game/Blueprints/UI/BPW_MainUI.UIEvent_ShowText` (`/Game/Blueprints/Player/BP_FirstPersionCharacter.MainUI` (`self.Player`)) (`self.Text Lins_LoreDontHasWight`) true 1.0 false)
              (elif true
                (`/Game/Blueprints/UI/BPW_MainUI.UIEvent_ShowText` (`/Game/Blueprints/Player/BP_FirstPersionCharacter.MainUI` (`self.Player`)) (`self.Text Lins_not lore on elevator`) true 1.0 false)))
            (else
              (`/Game/Blueprints/UI/BPW_MainUI.UIEvent_ShowText` (`/Game/Blueprints/Player/BP_FirstPersionCharacter.MainUI` (`self.Player`)) (`self.Text Lins_player not on Elevator`) true 1.0 false))))))))

(event `self.ReceiveBeginPlay`
  (`parent.ReceiveBeginPlay`)
  ; Debug
  (if (`KismetSystemLibrary.IsPackagedForDistribution`)
    (set `self.Debug` false)))

(fn `UserConstructionScript`
  (`parent.UserConstructionScript`))