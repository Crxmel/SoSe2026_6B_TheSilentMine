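; Child Blueprint of a generator-linked light that animates its point light intensity before and after the generator-on event.
; On BeginPlay, Timeline_1 drives intensity as a curve scaled by LightIntensity.
; GenonEvent, a one-shot because the parent unbinds it, waits TimelineStartDelay and then plays the turn-on curve.
; When that finishes, Timeline_1 stops and Timeline_0 takes over the intensity.
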(event `self.ReceiveBeginPlay`
  (`parent.ReceiveBeginPlay`)
  (bind (_direction _newtrack_0) (`Timeline|Timeline_1` :!label _label)
    (:`Update`
      (`LightComponent.SetIntensity` (`self.PointLight`) (* _newtrack_0 (`self.Light Intensity`))))))

(event `self.GenOn_Event`
  ; einmaliger trigger für event weil im parent das event geunbindet wird
  (`parent.GenOn_Event`)
  (`KismetSystemLibrary.Delay` (`self.TimelineStart_Delay`))
  (bind (_direction _oncurve) (`Timeline|Timeline`)
    (:`Update`
      (`LightComponent.SetIntensity` (`self.PointLight`) (* _oncurve (`self.Light Intensity`))))
    (:`Finished`
      (`|ExecutionSequence`
        (:`then_0`
          (goto _label :!via `Stop`))
        (:`then_1`
          (bind (_direction_2 _newtrack_0) (`Timeline|Timeline_0`)
            (:`Update`
              (`LightComponent.SetIntensity` (`self.PointLight`) (* _newtrack_0 (`self.Light Intensity`))))))))))

(fn `UserConstructionScript`
  (`parent.UserConstructionScript`))