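; An interactable generator Blueprint that the player can switch on.
; On player interaction it plays its motor sound component from the start and calls the generator-on dispatcher or event.
; BeginPlay handles a lighting debug flag, forcing it off in packaged distribution builds and otherwise printing an on-screen notice when it is enabled.
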(event `self.ReceiveBeginPlay`
  ;[0.15 0.07453 0 0.5] Debug
  (if (`KismetSystemLibrary.IsPackagedForDistribution`)
    (set `self.LighteDebug` false)
    (elif (`self.LighteDebug`)
      (`KismetSystemLibrary.PrintString` (`KismetStringLibrary.Concat_StrStr` "Lightning-Debug in " (`KismetSystemLibrary.GetDisplayName` self) " is on") true true (struct :`R` 1.0 :`G` 0.361202 :`A` 0.504348) 7.0))))

(event `self.PlayerInteract`
  (`AudioComponent.Play` (`self.SC_Motor1`) 0.0)
  (`self.GenOn`))

(fn `UserConstructionScript`
  (`parent.UserConstructionScript`))