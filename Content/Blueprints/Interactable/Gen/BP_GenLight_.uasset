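; BP_GenLight_ is a point light actor tied to a referenced generator Blueprint, BPGen.
; On BeginPlay it binds to the generator's GenOn dispatcher and zeroes the light's intensity unless the generator's LighteDebug flag is set.
; A missing reference prints a warning and tints the light red.
; The GenOn handler is empty, so nothing here relights it, and the unbind call is unconnected.
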(event `self.ReceiveBeginPlay`
  (bind _bp_gen (`self.BP_Gen`))
  (`/Engine/EditorBlueprintResources/StandardMacros.IsValid` _bp_gen
    (:`Is Valid`
      (add `/Game/Blueprints/Interactable/Gen/BP_Interactable_Generator.GenOn` _bp_gen (delegate `GenOn_Event`))
      (if (not (`/Game/Blueprints/Interactable/Gen/BP_Interactable_Generator.LighteDebug` _bp_gen))
        (`LightComponent.SetIntensity` (`self.PointLight`) 0.0)))
    (:`Is Not Valid`
      ;[0.15 0.07192 0 0.5] Debug
      (`KismetSystemLibrary.PrintString` (`KismetStringLibrary.Concat_StrStr` (`KismetSystemLibrary.GetDisplayName` self) " need ref to BP_gen") true true (struct :`R` 1.0 :`B` 0.011229 :`A` 1.0))
      (`LightComponent.SetLightColor` (`self.PointLight`) (struct :`R` 1.0 :`B` 0.117004 :`A` 1.0) true))))

(event `GenOn_Event`)

(fn `UserConstructionScript`)