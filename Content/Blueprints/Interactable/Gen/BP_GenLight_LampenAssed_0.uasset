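; Generator-driven lamp that lights up when its parent's GenonEvent fires, then keeps its point light on a flicker curve.
; On BeginPlay it creates a dynamic material from the lamp mesh, whose emissive color is set after a start delay on the event.
; A startup timeline ramps light intensity, then hands over to a second timeline that plays a flicker sound on dips, throttled by a DoOnce.
; The trigger is one-shot because the parent unbinds the event.
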(event `self.ReceiveBeginPlay`
  (`parent.ReceiveBeginPlay`)
  (bind _returnvalue (`KismetMaterialLibrary.CreateDynamicMaterialInstance` (`PrimitiveComponent.GetMaterial` (`self.SM_Lampe`) 1) "EmissiveColor"))
  (set `self.DynamicMaterial` _returnvalue))

(event `self.GenOn_Event`
  ; einmaliger trigger für event weil im parent das event geunbindet wird
  (`parent.GenOn_Event`)
  (`KismetSystemLibrary.Delay` (`self.TimelineStart_Delay`))
  (`MaterialInstanceDynamic.SetVectorParameterValue` (`self.DynamicMaterial`) "EmissiveColor" (`self.Value`))
  (bind (_direction _oncurve) (`Timeline|LightingTimelin`)
    (:`Update`
      (`LightComponent.SetIntensity` (`self.PointLight`) (* _oncurve (`self.Light Intensity`))))
    (:`Finished`
      (bind (_direction_2 _newtrack_0) (`Timeline|Timeline` :!via `PlayFromStart`)
        (:`Update`
          (`LightComponent.SetIntensity` (`self.PointLight`) (* _newtrack_0 (`self.Light Intensity`)))
          (if (< _newtrack_0 0.9)
            (`/Engine/EditorBlueprintResources/StandardMacros.DoOnce` false :!label _label
              (:`Completed`
                (`AudioComponent.Play` (`self.SC_flickering_lamps`) 0.0)
                (`KismetSystemLibrary.Delay` 3.0)
                (goto _label :!via `Reset`)))))))))

(fn `UserConstructionScript`
  (`parent.UserConstructionScript`))