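; BP_Interactable_Stone is an interactable stone that blocks the BP_Lore actor and can be removed by a player who has a pickaxe.
; On begin overlap it caches BP_Lore, sets its StoneInFrontFromSpline1 flag and calls StopLorenAnimation1.
; End overlap with that cached actor clears the flag.
; PlayerInteract destroys the stone only when the player's HasPickaxe is true.
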(event `self.ReceiveActorEndOverlap`
  (params (OtherActor :type "Actor Object Reference"))
  (`parent.ReceiveActorEndOverlap` OtherActor)
  (if (== OtherActor (`self.As BP Lore`))
    (set `/Game/Blueprints/Lore/BP_Lore.StoneInFrontFromSpline1` false (`self.As BP Lore`))))

(event `self.ReceiveActorBeginOverlap`
  (params (OtherActor :type "Actor Object Reference"))
  (`parent.ReceiveActorBeginOverlap` OtherActor)
  (`/Engine/EditorBlueprintResources/StandardMacros.IsValid` (`self.As BP Lore`)
    (:`Is Valid`
      (if (== (`self.As BP Lore`) OtherActor)
        (set `/Game/Blueprints/Lore/BP_Lore.StoneInFrontFromSpline1` true (stale _output_get) :!label _label)
        (`/Game/Blueprints/Lore/BP_Lore.StopLorenAnimation_1` (stale _output_get))))
    (:`Is Not Valid`
      (bind _asbp_lore (cast `/Game/Blueprints/Lore/BP_Lore` OtherActor))
      (bind _output_get (set `self.As BP Lore` _asbp_lore))
      (goto _label))))

(event `self.PlayerInteract`
  (if (`/Game/Blueprints/Player/BP_FirstPersionCharacter.HasPickaxe` (`self.Player`))
    (`self.K2_DestroyActor`)))

(fn `UserConstructionScript`
  (`parent.UserConstructionScript`))