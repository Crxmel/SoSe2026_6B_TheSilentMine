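; First-person player character that handles walking, looking, pausing and interaction, and creates the main UI and cave ambience on BeginPlay.
; Movement and look respect InputBlock, with timed footsteps chosen by a downward trace's physical surface.
; A short camera sphere trace calls BPI_Interact on hit actors, gated by a DoOnce that camera input also resets to avoid getting stuck.
; Debug mode, disabled in distribution builds, changes movement scale, draws traces and allows destroying targeted actors.
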(event `self.ReceiveBeginPlay`
  (`|ExecutionSequence`
    (:`then_0`
      (if (`KismetSystemLibrary.IsPackagedForDistribution`)
        (set `self.Debug` false)))
    (:`then_1`
      (bind _returnvalue (`|CreateWidget` "/Game/Blueprints/UI/BPW_MainUI.BPW_MainUI_C" (`GameplayStatics.GetPlayerController` 0)))
      (bind _output_get (set `self.MainUI` _returnvalue))
      (`UserWidget.AddToPlayerScreen` _output_get 0)
      (`/Game/Blueprints/UI/BPW_MainUI.SetPlayerVariableInMainUI` (`self.MainUI`) self)
      (`GameplayStatics.PlaySound2D` "/Game/Sounds/Roh/WeLoveIndies/Atmo/atmo-cave-cave-loop-01.atmo-cave-cave-loop-01" 1.0 1.0 0.0 null null))))

(event `EnhancedInput|/Game/Controls/Inputs/Player/IA_Move`
  (params (ActionValue :type "Vector2D Structure") (ElapsedSeconds :type "Float (double-precision)") (TriggeredSeconds :type "Float (double-precision)") (InputAction :type "InputAction Object Reference" :default "/Game/Controls/Inputs/Player/IA_Move.IA_Move"))
  (bind _returnvalue (select `bool` (`self.Debug`) :`false` (`self.Walkspeed`) :`true` 1.5))
  ; Walk
  (:`Triggered`
    (if (not (`self.InputBlock`))
      (`|ExecutionSequence`
        (:`then_0`
          ;; Stepsoundtrigger
          (`/Engine/EditorBlueprintResources/StandardMacros.DoOnce` false :!label _label
            (:`Completed`
              (`self.WalkSounds`)
              (`KismetSystemLibrary.Delay` (`self.StepsoundDelay`))
              (goto _label :!via `Reset`))))
        (:`then_1`
          (`self.Move` (* ActionValue_X _returnvalue) (* _returnvalue ActionValue_Y)))))))

(event `EnhancedInput|/Game/Controls/Inputs/Player/IA_RotateCamera`
  (params (ActionValue :type "Vector2D Structure") (ElapsedSeconds :type "Float (double-precision)") (TriggeredSeconds :type "Float (double-precision)") (InputAction :type "InputAction Object Reference" :default "/Game/Controls/Inputs/Player/IA_RotateCamera.IA_RotateCamera"))
  (bind _maussensetiv (`self.Maussensetiv`))
  (:`Triggered`
    (if (not (`self.InputBlock`))
      (`self.AddControllerYawInput` (* ActionValue_X _maussensetiv))
      (`self.AddControllerPitchInput` (* _maussensetiv ActionValue_Y))
      (`KismetSystemLibrary.Delay` 0.5)
      (`self.ResetLMBinput`))))

(event `EnhancedInput|/Game/Controls/Inputs/Player/IA_Interact`
  (params (ActionValue :type Boolean) (ElapsedSeconds :type "Float (double-precision)") (TriggeredSeconds :type "Float (double-precision)") (InputAction :type "InputAction Object Reference" :default "/Game/Controls/Inputs/Player/IA_Interact.IA_Interact"))
  (:`Triggered`
    ; damit man nicht stuck ist wenn man mit LMB den negsten teztbox macht
    (`/Engine/EditorBlueprintResources/StandardMacros.DoOnce` false :!label _label_2
      (:`Completed`
        (`self.Interact`)
        (if (not (`self.InputBlock`))
          (goto _label_2 :!via `Reset`))))))

(event `ResetLMBinput`
  (goto _label_2 :!via `Reset`))

(event `EnhancedInput|/Game/Controls/Inputs/Player/IA_Paused`
  (params (ActionValue :type Boolean) (ElapsedSeconds :type "Float (double-precision)") (TriggeredSeconds :type "Float (double-precision)") (InputAction :type "InputAction Object Reference" :default "/Game/Controls/Inputs/Player/IA_Paused.IA_Paused"))
  (:`Triggered`
    (`/Game/Blueprints/UI/BPW_MainUI.PressPaused` (`self.MainUI`))))

(event `WalkSounds`
  (bind _returnvalue (`self.K2_GetActorLocation` (`GameplayStatics.GetPlayerPawn` 0)))
  (bind (_outhit _returnvalue_2) (`KismetSystemLibrary.SphereTraceSingle` _returnvalue (+ _returnvalue (0.0 0.0 -100.0)) 0.0 "TraceTypeQuery1"))
  (if _returnvalue_2
    (bind (_bblockinghit _binitialoverlap _time _distance _location _impactpoint _normal _impactnormal _physmat) (`GameplayStatics.BreakHitResult` _outhit))
    (`GameplayStatics.PlaySoundAtLocation` (select `EPhysicalSurface` (`PhysicalMaterial.SurfaceType` _physmat) :`SurfaceType_Default` "/Game/Sounds/SC_DirtSteps.SC_DirtSteps" :`SurfaceType1` "/Game/Sounds/SC_WoodSteps.SC_WoodSteps" :`SurfaceType2` "/Game/Sounds/SC_DirtSteps.SC_DirtSteps" :!type "SoundBase Object Reference") _location (struct) 1.0 1.0 0.0 null null null null)))

(event `EnhancedInput|/Game/Controls/Inputs/Player/IA_DebugEnf`
  (params (ActionValue :type Boolean) (ElapsedSeconds :type "Float (double-precision)") (TriggeredSeconds :type "Float (double-precision)") (InputAction :type "InputAction Object Reference" :default "/Game/Controls/Inputs/Player/IA_DebugEnf.IA_DebugEnf"))
  (bind _camera (`self.Camera`))
  (bind _returnvalue (`SceneComponent.K2_GetComponentLocation` _camera))
  (:`Triggered`
    (if (`self.Debug`)
      (bind (_outhit _returnvalue_2) (`KismetSystemLibrary.SphereTraceSingleForObjects` :`Start` _returnvalue :`End` (+ _returnvalue (* (`SceneComponent.GetForwardVector` _camera) 150.0)) :`Radius` 1.0 :`ObjectTypes` (`|MakeArray` "ObjectTypeQuery1" "ObjectTypeQuery2" "ObjectTypeQuery3" "ObjectTypeQuery4" :!type "EObjectTypeQuery Enum") :`DrawDebugType` "ForDuration" :`DrawTime` 2.0))
      (if _returnvalue_2
        (`self.K2_DestroyActor` (`.HitActor` (`GameplayStatics.BreakHitResult` _outhit)))))))

(fn `Interact`
  (bind _camera (`self.Camera`))
  (bind _returnvalue (`SceneComponent.K2_GetComponentLocation` _camera))
  (bind (_outhit _returnvalue_2) (`KismetSystemLibrary.SphereTraceSingleForObjects` :`Start` _returnvalue :`End` (+ _returnvalue (* (`SceneComponent.GetForwardVector` _camera) 150.0)) :`Radius` 1.0 :`ObjectTypes` (`|MakeArray` "ObjectTypeQuery1" "ObjectTypeQuery2" "ObjectTypeQuery3" "ObjectTypeQuery4" :!type "EObjectTypeQuery Enum") :`DrawDebugType` (select `bool` (`self.Debug`) :`true` "ForDuration" :!type "EDrawDebugTrace Enum") :`DrawTime` 2.0))
  (if _returnvalue_2
    (bind (_bblockinghit _binitialoverlap _time _distance _location _impactpoint _normal _impactnormal _physmat _hitactor) (`GameplayStatics.BreakHitResult` _outhit))
    (if (`KismetSystemLibrary.DoesImplementInterface` _hitactor "/Game/Blueprints/BPI_Interact.BPI_Interact_C")
      (message `/Game/Blueprints/BPI_Interact.Interact` _hitactor self))))

(fn `Move`
  (params (`Left / Right` :type "Float (double-precision)") (`Forward / Backward` :type "Float (double-precision)"))
  (`self.AddMovementInput` (`self.GetActorForwardVector`) `Left / Right`)
  (`self.AddMovementInput` (`self.GetActorRightVector`) `Forward / Backward`))

(fn `UserConstructionScript`)