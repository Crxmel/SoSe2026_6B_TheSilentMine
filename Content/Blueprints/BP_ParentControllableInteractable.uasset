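; Parent Blueprint for interactable pawns that the player can take control of and later leave to return to the character.
; Interacting blends the view target to this pawn and possesses it.
; Returning places the character on ground found by a downward line trace from a respawn point or the camera, then blends back and repossesses it.
; Debug arrows are always hidden in packaged builds.
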(event `self.ReceiveBeginPlay`
  ; Debug
  (if (`KismetSystemLibrary.IsPackagedForDistribution`)
    (set `self.Debug` false)
    (`SceneComponent.SetVisibility` (`self.Arrow`) false false)
    (`SceneComponent.SetVisibility` (`self.Arrow1`) false false)
    (else
      (`SceneComponent.SetVisibility` (`self.Arrow`) (`self.Debug`) false)
      (`SceneComponent.SetVisibility` (`self.Arrow1`) (`self.Debug`) false))))

(event `PlayerInteract`
  (`self.GetPosses` self))

(event `GetPosses`
  (params (`In Pawn` :type "Pawn Object Reference"))
  (set `self.In Pawn` `In Pawn`)
  (`PlayerController.SetViewTargetWithBlend` (`GameplayStatics.GetPlayerController` 0) (`self.In Pawn`) (`self.Smooth Prosess Duration`) (`self.Blend Func`) (`self.SmoothPossessBlendExp`) true)
  (`Controller.Possess` (`GameplayStatics.GetPlayerController` 0) (`self.In Pawn`)))

(event `Return to Charakter`
  (`self.PositionPlayerCharakter`)
  (`PlayerController.SetViewTargetWithBlend` (`GameplayStatics.GetPlayerController` 0) (`self.Player`) (`self.Smooth Prosess Duration`) (`self.Blend Func`) (`self.SmoothPossessBlendExp`) true)
  (`Controller.Possess` (`GameplayStatics.GetPlayerController` 0) (`self.Player`))
  (set `self.In Pawn` null))

(fn `Interact`
  (params (Player :type "/Game/Blueprints/Player/BP_FirstPersionCharacter Object Reference"))
  (returns (PlayerInputBlock :type Boolean))
  (`/Engine/EditorBlueprintResources/StandardMacros.IsValid` (`self.Player`)
    (:`Is Valid`
      _)
    (:`Is Not Valid`
      (set `self.Player` Player)))
  (`self.PlayerInteract`)
  (return false))

(fn `PositionPlayerCharakter`
  (locals (Cam :type "CameraComponent Object Reference"))
  (bind _returnvalue (`SceneComponent.K2_GetComponentLocation` (select `bool` (`self.Spawn on Respawnpoint`) :`false` (`local.Cam`) :`true` (`self.Respawnpoint_1`) :!type "SceneComponent Object Reference")))
  (bind _output_get (set `local.Cam` (`self.Camera_1`)))
  (`/Engine/EditorBlueprintResources/StandardMacros.IsValid` _output_get
    (:`Is Valid`
      (bind (_outhit _returnvalue_2) (`KismetSystemLibrary.LineTraceSingleForObjects` :`Start` _returnvalue :`End` (- _returnvalue (0.0 0.0 300.0)) :`ObjectTypes` (`|MakeArray` "ObjectTypeQuery1" "ObjectTypeQuery2" :!type "EObjectTypeQuery Enum") :`DrawDebugType` (select `bool` (`self.Debug`) :`false` "ForDuration" :!type "EDrawDebugTrace Enum")))
      (if _returnvalue_2
        (`self.K2_SetActorLocationAndRotation` (`self.Player`) (+ (`.Location` (`GameplayStatics.BreakHitResult` _outhit)) (`KismetMathLibrary.MakeVector` 0.0 0.0 (+ (`CapsuleComponent.CapsuleHalfHeight` (`Character.CapsuleComponent` (`self.Player`))) 1.0))) (`SceneComponent.K2_GetComponentRotation` (`local.Cam`)) false false)))))

(fn `UserConstructionScript`
  (if (`KismetSystemLibrary.IsPackagedForDistribution`)
    (set `self.Debug` false)
    (`SceneComponent.SetVisibility` (`self.Arrow`) false false)
    (`SceneComponent.SetVisibility` (`self.Arrow1`) false false)
    (else
      (`SceneComponent.SetVisibility` (`self.Arrow`) (`self.Debug`) false)
      (`SceneComponent.SetVisibility` (`self.Arrow1`) (`self.Debug`) false))))