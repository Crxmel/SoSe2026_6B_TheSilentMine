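; Grate door puzzle actor that the player rigs by tying a rope (Seil) to the door and to a cart (Lore).
; Each interaction requires the rope and reveals rope meshes; interacting with the door without it shows UI text.
; Once both ends are connected, the Stopper actor is destroyed, while a separate OpenDoor event removes the gate components.
; A debug flag deletes the door on BeginPlay outside distribution builds.
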(event `self.ReceiveBeginPlay`
  (if (`KismetSystemLibrary.IsPackagedForDistribution`)
    (set `self.Debug_OpenDoor` false)
    (elif (`self.Debug_OpenDoor`)
      (`self.K2_DestroyActor`))))

(event `self.PlayerInteract`
  (if (`/Game/Blueprints/Player/BP_FirstPersionCharacter.HasSeil` (`self.Player`))
    (`SceneComponent.SetVisibility` (`self.Cylinder_AADE4D53`) true false)
    (`SceneComponent.SetVisibility` (`self.Cylinder_AADE4D54`) true false)
    (`SceneComponent.SetVisibility` (`self.Cylinder_AADE4D55`) true false)
    (`SceneComponent.SetVisibility` (`self.Cylinder_AADE4D56`) true false)
    (`SceneComponent.SetVisibility` (`self.Cylinder_AADE4D52`) true false)
    (`SceneComponent.SetVisibility` (`self.SM_Schlauch`) true false)
    (bind _output_get (set `self.ConectToDoor` true))
    (if (and _output_get (stale `interactWithLohre` _output_get_2) true) :!label _label
      (`/Engine/EditorBlueprintResources/StandardMacros.IsValid` (`self.Stopper`)
        (:`Is Valid`
          (`self.K2_DestroyActor` (`self.Stopper`)))))
    (else
      (`/Game/Blueprints/UI/BPW_MainUI.UIEvent_ShowText` (`/Game/Blueprints/Player/BP_FirstPersionCharacter.MainUI` (`self.Player`)) (`self.Text Lins`) true))))

(event `interactWithLohre`
  (params (Player :type "/Game/Blueprints/Player/BP_FirstPersionCharacter Object Reference"))
  (bind _output_get (set `self.Player` Player))
  (if (`/Game/Blueprints/Player/BP_FirstPersionCharacter.HasSeil` _output_get)
    (`SceneComponent.SetVisibility` (`self.Cylinder_AADE4D58`) true false)
    (`SceneComponent.SetVisibility` (`self.Cylinder_AADE4D57`) true false)
    (`SceneComponent.SetVisibility` (`self.Cylinder_AADE4D59`) true false)
    (`SceneComponent.SetVisibility` (`self.SM_Schlauch`) true false)
    (bind _output_get_2 (set `self.ConectToLore` true))
    (goto _label)))

(event `OpenDoor`
  (`ActorComponent.K2_DestroyComponent` (`self.SM_GitterTor`))
  (`ActorComponent.K2_DestroyComponent` (`self.Cylinder_AADE4D56`))
  (`ActorComponent.K2_DestroyComponent` (`self.Cylinder_AADE4D55`)))

(fn `UserConstructionScript`)