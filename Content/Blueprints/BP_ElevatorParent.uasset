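; Parent Blueprint for an elevator that works with a lever and can move a BP_Lore actor along with it.
; On lever interaction, two boxes detect the Lore and player, setting the lever's flags for player presence and Lore weight.
; PlayAnimation drives a timeline that offsets the elevator's height from its start, while adding the offset to the cached Lore's current height.
; AnimationFinish is an empty event called when the timeline finishes.
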(event `self.ReceiveBeginPlay`
  (set `self.WorldLocation` (`SceneComponent.K2_GetComponentLocation` (`self.DefaultSceneRoot`)))
  ; Debug
  (if (`KismetSystemLibrary.IsPackagedForDistribution`)
    (set `self.Debug` false)))

(event `InteractWithLever`
  (params (Lever :type "/Game/Blueprints/Interactable/BP_Interactable_elevatorLever Object Reference"))
  (bind _lever (`self.Lever`))
  (`/Engine/EditorBlueprintResources/StandardMacros.IsValid` (`self.Lever`)
    (:`Is Valid`
      _)
    (:`Is Not Valid`
      (set `self.Lever` Lever)))
  (set `/Game/Blueprints/Interactable/BP_Interactable_elevatorLever.PlayerOnElevator` false (`self.Lever`))
  (for _array_element (`PrimitiveComponent.GetOverlappingActors` (`self.Box`) "/Game/Blueprints/Lore/BP_Lore.BP_Lore_C")
    (bind _asbp_lore (cast `/Game/Blueprints/Lore/BP_Lore` _array_element)
      (:`then`
        (bind _output_get (set `self.As BP Lore` _asbp_lore))
        (if (`/Game/Blueprints/Lore/BP_Lore.LoreHasweight` _output_get)
          (set `/Game/Blueprints/Interactable/BP_Interactable_elevatorLever.LoreOnElevatorAndHasWight` true (`self.Lever`))
          (set `/Game/Blueprints/Interactable/BP_Interactable_elevatorLever.LoreOnElevatorAnd_DONT_HasWight` false (`self.Lever`))
          (else
            (set `/Game/Blueprints/Interactable/BP_Interactable_elevatorLever.LoreOnElevatorAnd_DONT_HasWight` true (`self.Lever`))
            (set `/Game/Blueprints/Interactable/BP_Interactable_elevatorLever.LoreOnElevatorAndHasWight` false (`self.Lever`)))))
      (:`CastFailed`
        (set `/Game/Blueprints/Interactable/BP_Interactable_elevatorLever.LoreOnElevatorAnd_DONT_HasWight` false _lever)
        (set `/Game/Blueprints/Interactable/BP_Interactable_elevatorLever.LoreOnElevatorAndHasWight` false _lever))))
  (for _array_element_2 (`PrimitiveComponent.GetOverlappingActors` (`self.Box1`) "/Game/Blueprints/Player/BP_FirstPersionCharacter.BP_FirstPersionCharacter_C")
    (cast `/Game/Blueprints/Player/BP_FirstPersionCharacter` _array_element_2)
    (set `/Game/Blueprints/Interactable/BP_Interactable_elevatorLever.PlayerOnElevator` true (`self.Lever`))))

(event `AnimationFinish`)

(event `PlayAnimation`
  (bind (_worldlocation_x _worldlocation_y _worldlocation_z) (`KismetMathLibrary.BreakVector` (`self.WorldLocation`)))
  (bind _as_bp_lore (`self.As BP Lore`))
  (bind _rootcomponent (`Actor.RootComponent` _as_bp_lore))
  (bind (_returnvalue_x _returnvalue_y _returnvalue_z) (`KismetMathLibrary.BreakVector` (`SceneComponent.K2_GetComponentLocation` _rootcomponent)))
  (bind (_direction _newtrack_0) (`Timeline|Timeline`)
    (:`Update`
      (bind _returnvalue (* _newtrack_0 (`self.AnimationsHoehe`)))
      (`SceneComponent.K2_SetWorldLocation` (`self.DefaultSceneRoot`) (`KismetMathLibrary.MakeVector` _worldlocation_x _worldlocation_y (+ _worldlocation_z _returnvalue)) false false :!label _label)
      (`/Engine/EditorBlueprintResources/StandardMacros.IsValid` _as_bp_lore
        (:`Is Valid`
          (`SceneComponent.K2_SetWorldLocation` _rootcomponent (`KismetMathLibrary.MakeVector` _returnvalue_x _returnvalue_y (+ _returnvalue_z _returnvalue)) false false))))
    (:`Finished`
      (`|ExecutionSequence`
        (:`then_0`
          (`self.AnimationFinish`))
        (:`then_1`
          (goto _label))))))

(fn `UserConstructionScript`)