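; BP_LorenRotation is a lever-operated turntable that rotates a cart (BP_Lore) and switches it to another spline track.
; A capsule trace finds the cart, and pawn checks at two scene points must be clear.
; The cart then snaps into place, the lever animates, sound plays and a timeline rotates platform and cart forward or backward by current spline.
; Player interaction is disabled until the timeline finishes and changes the spline.
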(event `InteractWithHebel_Event`
  (params (Hebel :type "/Game/Blueprints/Lore/BP_LorenRotationHebel Object Reference"))
  (bind _as_bp_lore (`self.As BP Lore`))
  (bind _sm_drehplattformmitte (`self.SM_DrehPlattformMitte`))
  (bind _as_bp_lore_2 (`self.As BP Lore`))
  (bind _returnvalue (`SceneComponent.K2_GetComponentLocation` (`self.SceneF`)))
  (bind _returnvalue_2 (`SceneComponent.K2_GetComponentLocation` (`self.SceneB`)))
  (bind _returnvalue_3 (`SceneComponent.K2_GetComponentLocation` _sm_drehplattformmitte))
  (bind (_returnvalue_x _returnvalue_y _returnvalue_z) (`KismetMathLibrary.BreakVector` (`SceneComponent.K2_GetComponentLocation` (`self.Lorensnap`))))
  (bind _returnvalue_4 (== (`/Game/Blueprints/Lore/BP_Lore.Move On Spline Mount` _as_bp_lore) (`self.SplineNumberByBeginPlay`)))
  (`/Engine/EditorBlueprintResources/StandardMacros.IsValid` (`self.Hebel`)
    (:`Is Valid`
      _)
    (:`Is Not Valid`
      (set `self.Hebel` Hebel)))
  (bind (_outhit _returnvalue_5) (`KismetSystemLibrary.CapsuleTraceSingleForObjects` :`Start` (+ _returnvalue_3 (0.0 0.0 1.0)) :`End` (+ _returnvalue_3 (* (`SceneComponent.GetUpVector` _sm_drehplattformmitte) 200.0)) :`ObjectTypes` (`|MakeArray` "ObjectTypeQuery2" :!type "EObjectTypeQuery Enum") :`DrawDebugType` "ForDuration" :`DrawTime` 2.0))
  (if _returnvalue_5
    (`/Engine/EditorBlueprintResources/StandardMacros.IsValid` (`self.As BP Lore`)
      (:`Is Valid`
        _)
      (:`Is Not Valid`
        (bind _asbp_lore (cast `/Game/Blueprints/Lore/BP_Lore` (`.HitActor` (`GameplayStatics.BreakHitResult` _outhit))))
        (set `self.As BP Lore` _asbp_lore)))
    ; is Lore on RotationsPlatform
    (bind (_outhit_2 _returnvalue_6) (`KismetSystemLibrary.CapsuleTraceSingleForObjects` :`Start` _returnvalue_2 :`End` _returnvalue_2 :`Radius` 10.0 :`ObjectTypes` (`|MakeArray` "ObjectTypeQuery3" :!type "EObjectTypeQuery Enum") :`DrawDebugType` "ForDuration" :`DrawTime` 2.0))
    (if (not _returnvalue_6)
      (bind (_outhit_3 _returnvalue_7) (`KismetSystemLibrary.CapsuleTraceSingleForObjects` :`Start` _returnvalue :`End` _returnvalue :`Radius` 10.0 :`ObjectTypes` (`|MakeArray` "ObjectTypeQuery3" :!type "EObjectTypeQuery Enum") :`DrawDebugType` "ForDuration" :`DrawTime` 2.0))
      (if (not _returnvalue_7)
        ; Lorenlocation for rotation
        (`self.K2_SetActorLocation` (`self.As BP Lore`) (`KismetMathLibrary.MakeVector` _returnvalue_x _returnvalue_y (+ _returnvalue_z 60.0)) false false)
        (set `/Game/Blueprints/Lore/BP_Lore.PlayerCanInteract` false _as_bp_lore)
        (`/Game/Blueprints/Lore/BP_LorenRotationHebel.PlayHebelAni` (`self.Hebel`))
        (`KismetSystemLibrary.Delay` 0.75)
        (`AudioComponent.Play` (`self.SC_Drehplattform`) 0.0)
        (if _returnvalue_4
          (bind (_direction _rotation _rotation2) (`Timeline|Timeline` :!via `PlayFromStart` :!label _label)
            (:`Update`
              (`self.K2_SetActorRotation` (`self.As BP Lore`) (`KismetMathLibrary.MakeRotator` 0.0 0.0 (* _rotation2 -90.0)) false)
              (`self.K2_SetActorRotation` (`KismetMathLibrary.MakeRotator` 0.0 0.0 (* _rotation 90.0))))
            (:`Finished`
              (set `/Game/Blueprints/Lore/BP_Lore.PlayerCanInteract` true _as_bp_lore_2)
              (`/Game/Blueprints/Lore/BP_Lore.ChangeSpline` _as_bp_lore_2 (`KismetMathLibrary.SelectInt` (`self.SplineNumberToChange`) (`self.SplineNumberByBeginPlay`) _returnvalue_4))))
          (else
            (goto _label :!via `ReverseFromEnd`)))))
    (else
      (`KismetSystemLibrary.PrintString` "False"))))

(fn `UserConstructionScript`)