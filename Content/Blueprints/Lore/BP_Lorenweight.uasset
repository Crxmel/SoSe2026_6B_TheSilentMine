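; BP_Lorenweight is an interactable weight object that the player, when carrying a pickaxe, can transfer onto a nearby BP_Lore actor.
; On interact, it runs a zero-length capsule trace at its own location, with persistent debug drawing, and casts the hit actor to BP_Lore.
; A successful hit flags that lore as weighted, reveals its stone mesh and destroys this actor.
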(event `self.PlayerInteract`
  (bind _returnvalue (`SceneComponent.K2_GetComponentLocation` (`self.Scene`)))
  (if (`/Game/Blueprints/Player/BP_FirstPersionCharacter.HasPickaxe` (`self.Player`))
    (bind (_outhit _returnvalue_2) (`KismetSystemLibrary.CapsuleTraceSingle` :`Start` _returnvalue :`End` _returnvalue :`Radius` 50.0 :`TraceChannel` "TraceTypeQuery1" :`DrawDebugType` "Persistent"))
    (if _returnvalue_2
      (bind _asbp_lore (cast `/Game/Blueprints/Lore/BP_Lore` (`.HitActor` (`GameplayStatics.BreakHitResult` _outhit))))
      (set `/Game/Blueprints/Lore/BP_Lore.LoreHasweight` true _asbp_lore)
      (`SceneComponent.SetVisibility` (`/Game/Blueprints/Lore/BP_Lore.Stone_NO_2_low` _asbp_lore) true false)
      (`self.K2_DestroyActor`))))

(fn `UserConstructionScript`)