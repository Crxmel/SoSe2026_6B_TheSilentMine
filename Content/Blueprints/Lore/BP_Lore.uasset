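; Player-moved mine cart (Lore) that rides along splines while the player interacts with it.
; The stand box the player occupies sets travel direction and camera mount, and move input plays or reverses that spline's timeline.
; ChangeSpline switches between two tracks, while the TotoLore variant uses its own timeline and can tip into physics, opening its Door.
; Surface-based footsteps loop during movement via a downward trace, marked unfinished.
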(event `self.PlayerInteract`
  ; JoinDeJoin
  ;; controllirt wo player steht
  (if (`/Game/Blueprints/Player/BP_FirstPersionCharacter.InputBlock` (`self.Player`))
    _
    (elif (`self.PlayerCanInteract`)
      (if (`self.IsTotoLore`)
        (`/Game/Blueprints/BP_GitterTuer.interactWithLohre` (`self.Door`) (`self.Player`))
        (else
          (`|ExecutionSequence`
            (:`then_0`
              _))))
      (`|ExecutionSequence`
        (:`then_0`
          (bind _returnvalue (`self.GetColliderPlayerInStand` (`self.Box`)))
          (if _returnvalue
            (set `self.SetRespawnOn` false)
            (`SceneComponent.K2_AttachToComponent` (`self.Camera_1`) (select `bool` (`self.SetRespawnOn`) :`false` (`self.CamPosi_2`) :`true` (`self.CamPosi_1`)) "None" "KeepRelative" "KeepRelative" "KeepRelative" true :!label _label)
            (`SceneComponent.SetVisibility` (`/Game/Blueprints/Player/BP_FirstPersionCharacter.SpotLight` (`self.Player`)) false false)
            (`SceneComponent.SetVisibility` (`self.SpotLight`) true false)
            (`parent.PlayerInteract`)))
        (:`then_1`
          (bind _returnvalue_2 (`self.GetColliderPlayerInStand` (`self.Box1`)))
          (if _returnvalue_2
            (set `self.SetRespawnOn` true)
            (goto _label)))))))

(event `EnhancedInput|/Game/Controls/Inputs/Lore/IA_InteractCancel`
  (params (ActionValue :type Boolean) (ElapsedSeconds :type "Float (double-precision)") (TriggeredSeconds :type "Float (double-precision)") (InputAction :type "InputAction Object Reference" :default "/Game/Controls/Inputs/Lore/IA_InteractCancel.IA_InteractCancel"))
  ; JoinDeJoin
  (:`Triggered`
    (set `self.StepsoundStop` true :!label _label_2)
    (`SceneComponent.SetVisibility` (`/Game/Blueprints/Player/BP_FirstPersionCharacter.SpotLight` (`self.Player`)) true false)
    (`SceneComponent.SetVisibility` (`self.SpotLight`) false false)
    (`self.StopLoreAnimation_0`)
    (`self.StopLoreAnimation_1`)
    (`self.StopTotoLore`)
    (`KismetSystemLibrary.DelayUntilNextTick`)
    (`self.Return to Charakter`)))

(event `InteractWithLoreCanceld`
  ; JoinDeJoin
  (goto _label_2))

(event `TotoloreAnimation`
  ; TotoLore
  (`self.InteractWithLoreCanceld`)
  (set `self.PlayerCanInteract` false)
  (`KismetSystemLibrary.DelayUntilNextFrame`)
  (bind (_direction _forward _rotation) (`Timeline|Timeline_2` :!via `PlayFromStart`)
    (:`Update`
      (`self.K2_AddActorLocalOffset` (`KismetMathLibrary.MakeVector` (* _forward 1.0)))
      (`self.K2_AddActorWorldRotation` (`KismetMathLibrary.MakeRotator` 0.0 (* _rotation 90.0 (`GameplayStatics.GetWorldDeltaSeconds`)))))
    (:`Finished`
      (`PrimitiveComponent.SetSimulatePhysics` (`self.SM_Lore`) true)
      (`/Game/Blueprints/BP_GitterTuer.OpenDoor` (`self.Door`))
      (set `self.StepsoundStop` true))))

(event `StartTotoLore`
  (bind _spline (`/Game/Blueprints/Lore/BP_Spline.Spline` (`self.Spline_0`)))
  ; TotoLore
  (bind (_direction _newtrack_0) (`Timeline|Timeline_1` :!label _label_3)
    (:`Update`
      (bind _returnvalue (* _newtrack_0 (`SplineComponent.GetSplineLength` _spline)))
      (`self.K2_SetActorLocationAndRotation` (`SplineComponent.GetLocationAtDistanceAlongSpline` _spline _returnvalue "World") (`SplineComponent.GetRotationAtDistanceAlongSpline` _spline _returnvalue "World")))))

(event `EnhancedInput|/Game/Controls/Inputs/Lore/IA_LoreMoveForward`
  (params (ActionValue :type Boolean) (ElapsedSeconds :type "Float (double-precision)") (TriggeredSeconds :type "Float (double-precision)") (InputAction :type "InputAction Object Reference" :default "/Game/Controls/Inputs/Lore/IA_LoreMoveForward.IA_LoreMoveForward"))
  ; TotoLore
  (:`Triggered`
    (if (`self.IsTotoLore`)
      (if (not (`self.SetRespawnOn`))
        (if (not (`self.StopLohreSpline_1_Forward`))
          (goto _label_3))
        (else
          (goto _label_3 :!via `Reverse`))))))

(event `StopTotoLore`
  ; TotoLore
  (goto _label_3 :!via `Stop`))

(event `AktualisirungSpline_0`
  (bind _spline (`/Game/Blueprints/Lore/BP_Spline.Spline` (`self.Spline_0`)))
  ; Spline_0
  (bind (_direction _timelinelenght _time) (`Timeline|Timeline` :`NewTime` (stale `ChangeSpline_0` NewTime) :!label _label_4)
    (:`Update`
      (if (`self.Debug`)
        (`KismetSystemLibrary.PrintString` (`KismetStringLibrary.Conv_DoubleToString` _time) true true (struct :`R` 0.584079 :`G` 1.0 :`B` 0.14996 :`A` 0.501961) 5.0))
      (bind _returnvalue (* _timelinelenght (`SplineComponent.GetSplineLength` _spline)))
      (bind (_returnvalue_roll _returnvalue_pitch _returnvalue_yaw) (`KismetMathLibrary.BreakRotator` (`SplineComponent.GetRotationAtDistanceAlongSpline` _spline _returnvalue "World")))
      (`self.K2_SetActorLocationAndRotation` (`SplineComponent.GetLocationAtDistanceAlongSpline` _spline _returnvalue "World") (`KismetMathLibrary.MakeRotator` _returnvalue_roll _returnvalue_pitch _returnvalue_yaw)))))

(event `EnhancedInput|/Game/Controls/Inputs/Lore/IA_LoreMoveForward`
  (params (ActionValue :type Boolean) (ElapsedSeconds :type "Float (double-precision)") (TriggeredSeconds :type "Float (double-precision)") (InputAction :type "InputAction Object Reference" :default "/Game/Controls/Inputs/Lore/IA_LoreMoveForward.IA_LoreMoveForward"))
  ; Spline_0
  (:`Triggered`
    (if (`self.IsTotoLore`)
      _
      (elif (== (`self.Move On Spline Mount`) 0)
        (if (not (`self.SetRespawnOn`))
          (goto _label_4)
          (else
            (goto _label_4 :!via `Reverse`)))))))

(event `StopLoreAnimation_0`
  ; Spline_0
  (goto _label_4 :!via `Stop`))

(event `ChangeSpline_0`
  (params (NewTime :type "Float (single-precision)"))
  ; Spline_0
  (goto _label_4 :!via `SetNewTime`))

(event `AktualisirungSpline_1`
  (bind _spline (`/Game/Blueprints/Lore/BP_Spline.Spline` (`self.Spline_1`)))
  ; Spline_1
  (bind (_direction _newtrack_0 _time) (`Timeline|Timeline_0` :`NewTime` (stale `ChangeSpline_1` NewTime) :!label _label_5)
    (:`Update`
      (if (`self.Debug`)
        (`KismetSystemLibrary.PrintString` (`KismetStringLibrary.Conv_DoubleToString` _time) true true (struct :`R` 0.584079 :`G` 1.0 :`B` 0.14996 :`A` 0.501961) 5.0))
      (bind _returnvalue (* _newtrack_0 (`SplineComponent.GetSplineLength` _spline)))
      (bind (_returnvalue_roll _returnvalue_pitch _returnvalue_yaw) (`KismetMathLibrary.BreakRotator` (`SplineComponent.GetRotationAtDistanceAlongSpline` _spline _returnvalue "World")))
      (`self.K2_SetActorLocationAndRotation` (`SplineComponent.GetLocationAtDistanceAlongSpline` _spline _returnvalue "World") (`KismetMathLibrary.MakeRotator` _returnvalue_roll _returnvalue_pitch _returnvalue_yaw)))))

(event `EnhancedInput|/Game/Controls/Inputs/Lore/IA_LoreMoveForward`
  (params (ActionValue :type Boolean) (ElapsedSeconds :type "Float (double-precision)") (TriggeredSeconds :type "Float (double-precision)") (InputAction :type "InputAction Object Reference" :default "/Game/Controls/Inputs/Lore/IA_LoreMoveForward.IA_LoreMoveForward"))
  ; Spline_1
  (:`Triggered`
    (if (`self.IsTotoLore`)
      _
      (elif (== (`self.Move On Spline Mount`) 1)
        (if (not (`self.SetRespawnOn`))
          (goto _label_5)
          (elif (not (`self.StopLohreSpline_1_Forward`))
            (goto _label_5 :!via `Reverse`)))))))

(event `StopLoreAnimation_1`
  ; Spline_1
  (goto _label_5 :!via `Stop`))

(event `ChangeSpline_1`
  (params (NewTime :type "Float (single-precision)"))
  ; Spline_1
  (goto _label_5 :!via `SetNewTime`))

(event `ChangeSpline`
  (params (`Move On Spline Mount` :type Integer))
  ; Change Spline
  (bind _output_get (set `self.Move On Spline Mount` `Move On Spline Mount`))
  (switch `int` _output_get
    (:`0`
      (`self.ChangeSpline_0` 5.6)
      (`self.AktualisirungSpline_0`)
      (`KismetSystemLibrary.DelayUntilNextTick`)
      (`self.StopLoreAnimation_0`))
    (:`1`
      (`self.ChangeSpline_1` 8.9)
      (`self.AktualisirungSpline_1`)
      (`KismetSystemLibrary.DelayUntilNextTick`)
      (`self.StopLoreAnimation_1`))))

(event `EnhancedInput|/Game/Controls/Inputs/Lore/IA_LoreCancleMoveForward`
  (params (ActionValue :type Boolean) (ElapsedSeconds :type "Float (double-precision)") (TriggeredSeconds :type "Float (double-precision)") (InputAction :type "InputAction Object Reference" :default "/Game/Controls/Inputs/Lore/IA_LoreCancleMoveForward.IA_LoreCancleMoveForward"))
  ; StopAnimation
  (:`Triggered`
    (`self.StopLoreAnimation_0`)
    (`self.StopLoreAnimation_1`)
    (`self.StopTotoLore`)
    (set `self.StepsoundStop` true)))

(event `self.ReceiveBeginPlay`
  (`self.ChangeSpline_0` 0.0)
  (if (`self.IsTotoLore`)
    (`self.StartTotoLore`)
    (`KismetSystemLibrary.DelayUntilNextTick`)
    (`self.StopTotoLore`)))

(event `EnhancedInput|/Game/Controls/Inputs/Lore/IA_LoreMoveForward`
  (params (ActionValue :type Boolean) (ElapsedSeconds :type "Float (double-precision)") (TriggeredSeconds :type "Float (double-precision)") (InputAction :type "InputAction Object Reference" :default "/Game/Controls/Inputs/Lore/IA_LoreMoveForward.IA_LoreMoveForward"))
  (bind _returnvalue (`self.K2_GetActorLocation` (`GameplayStatics.GetPlayerPawn` 0)))
  ; sound noch nicht fertig
  (:`Triggered`
    (set `self.StepsoundStop` false)
    ;; Stepsoundtrigger
    (`|ExecutionSequence` :!label _label_6
      (:`then_0`
        (`KismetSystemLibrary.Delay` (`/Game/Blueprints/Player/BP_FirstPersionCharacter.StepsoundDelay` (`self.Player`)))
        (if (not (`self.StepsoundStop`))
          (goto _label_6)))
      (:`then_1`
        (bind (_outhit _returnvalue_2) (`KismetSystemLibrary.SphereTraceSingle` _returnvalue (+ _returnvalue (0.0 0.0 -100.0)) 0.0 "TraceTypeQuery1"))
        (if _returnvalue_2
          (bind (_bblockinghit _binitialoverlap _time _distance _location _impactpoint _normal _impactnormal _physmat) (`GameplayStatics.BreakHitResult` _outhit))
          (`GameplayStatics.PlaySoundAtLocation` (select `EPhysicalSurface` (`PhysicalMaterial.SurfaceType` _physmat) :`SurfaceType_Default` "/Game/Sounds/SC_DirtSteps.SC_DirtSteps" :`SurfaceType1` "/Game/Sounds/SC_WoodSteps.SC_WoodSteps" :`SurfaceType2` "/Game/Sounds/SC_DirtSteps.SC_DirtSteps" :!type "SoundBase Object Reference") _location (struct) 1.0 1.0 0.0 null null null null))))))

(fn `GetColliderPlayerInStand`
  (params (`Box Collision` :type "BoxComponent Object Reference"))
  (returns (ReturnValue :type Boolean))
  (bind (_outactors _returnvalue) (`KismetSystemLibrary.BoxOverlapActors` (`SceneComponent.K2_GetComponentLocation` `Box Collision`) (`BoxComponent.GetScaledBoxExtent` `Box Collision`) (`|MakeArray` "ObjectTypeQuery3" :!type "EObjectTypeQuery Enum")))
  (if _returnvalue
    (for _array_element _outactors
      (return (== _array_element (`self.Player`))))))

(fn `UserConstructionScript`
  (`parent.UserConstructionScript`))