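; BP_LorenRotationHebel is an interactable lever (Hebel) that operates a rotation platform once fitted with a handle.
; Interacting without a fitted handle reveals the lever mesh if the player carries one, otherwise the player's UI shows a text prompt.
; Once fitted, interaction passes the lever to RotationPlatform.InteractWithHebelEvent.
; A separate PlayHebelAni event alternates a timeline forward and backward through a FlipFlop to pitch the lever's scene component.
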(event `self.PlayerInteract`
  (bind _player (`self.Player`))
  ; Interact with Actor
  (if (`self.HasLever`)
    ;;[0.009307 0.15 0.003039 0.5] redy to Rotate
    (`/Game/Blueprints/Lore/BP_LorenRotation.InteractWithHebel_Event` (`self.RotationPlatform`) self)
    (else
      ;;[0 0.15 0.1484 0.5] Activate lever
      (if (`/Game/Blueprints/Player/BP_FirstPersionCharacter.HasLever` _player)
        (set `self.HasLever` true)
        (`SceneComponent.SetVisibility` (`self.SM_Lever`) true false)
        (else
          (`/Game/Blueprints/UI/BPW_MainUI.UIEvent_ShowText` (`/Game/Blueprints/Player/BP_FirstPersionCharacter.MainUI` _player) (`self.Text Lins`) true 1.0 false))))))

(event `PlayHebelAni`
  ; Animation
  (`/Engine/EditorBlueprintResources/StandardMacros.FlipFlop`
    (:`A`
      (bind (_direction _rotate) (`Timeline|Timeline` :!label _label)
        (:`Update`
          (`SceneComponent.K2_SetRelativeRotation` (`self.Scene`) (`KismetMathLibrary.MakeRotator` 0.0 (* _rotate 50.0)) false false))))
    (:`B`
      (goto _label :!via `Reverse`))))

(fn `UserConstructionScript`
  (`parent.UserConstructionScript`))