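; Mine cart (Lore) actor that the first-person player pushes back and forth along splines.
; On overlap, box checks at rear and front play or reverse timelines that place it on Spline0 or Spline1, with a front-stone block on Spline1.
; Changespline switches tracks and refreshes the position by briefly playing the timeline.
; The tutorial variant uses its own timeline, forwards interaction to a Door, and has a fall animation ending in physics and door opening.
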(event `self.ReceiveActorEndOverlap`
  (params (OtherActor :type "Actor Object Reference"))
  ; Animation stop
  (if (== OtherActor (`self.First Persion Character`))
    (`self.StopLorenAnimation_0`)
    (`self.StopLorenAnimation_1`)
    (`self.StopTotorialLore`)
    ; nur für tastencontroll im player
    (`/Engine/EditorBlueprintResources/StandardMacros.DoOnce` false
      (:`Completed`
        (`/Game/Blueprints/Player/BP_FirstPersionCharacter.SetLohre` (`self.First Persion Character`) self)))))

(event `TotoloreAnimation`
  ; Animation
  ;;[0.15 0.1304 0 0.5] LorenToto
  (bind (_direction _forward _rotation) (`Timeline|LorenfallAnimation` :!via `PlayFromStart`)
    (:`Update`
      (`self.K2_AddActorLocalOffset` (`KismetMathLibrary.MakeVector` (* _forward 1.0)))
      (`self.K2_AddActorWorldRotation` (`KismetMathLibrary.MakeRotator` 0.0 (* _rotation 90.0 (`GameplayStatics.GetWorldDeltaSeconds`)))))
    (:`Finished`
      (`PrimitiveComponent.SetSimulatePhysics` (`self.SM_Lore`) true)
      (`/Game/Blueprints/BP_GitterTuer.OpenDoor` (`self.Door`)))))

(event `StopTotorialLore`
  (bind _spline (`/Game/Blueprints/Lore/BP_Spline.Spline` (`self.Spline_0`)))
  ; Animation
  ;;[0.15 0.1304 0 0.5] LorenToto
  (bind (_direction _newtrack_0) (`Timeline|TotorialTimelin` :!via `Stop` :!label _label)
    (:`Update`
      (bind _returnvalue (* _newtrack_0 (`SplineComponent.GetSplineLength` _spline)))
      (`self.K2_SetActorLocationAndRotation` (`SplineComponent.GetLocationAtDistanceAlongSpline` _spline _returnvalue "World") (`SplineComponent.GetRotationAtDistanceAlongSpline` _spline _returnvalue "World")))))

(event `AktualisirungSpline0`
  (bind _spline (`/Game/Blueprints/Lore/BP_Spline.Spline` (`self.Spline_0`)))
  ; Animation
  (bind (_direction _timelinelenght) (`Timeline|Timeline` :`NewTime` (stale `ChangeTimeSpline_0` NewTime) :!label _label_2)
    (:`Update`
      (if (`self.Loren-Debug`)
        (`KismetSystemLibrary.PrintString` (`KismetStringLibrary.Conv_DoubleToString` _timelinelenght) true true (struct :`R` 0.584079 :`G` 1.0 :`B` 0.14996 :`A` 0.501961) 5.0))
      (bind _returnvalue (* _timelinelenght (`SplineComponent.GetSplineLength` _spline)))
      (`self.K2_SetActorLocationAndRotation` (`SplineComponent.GetLocationAtDistanceAlongSpline` _spline _returnvalue "World") (`SplineComponent.GetRotationAtDistanceAlongSpline` _spline _returnvalue "World")))))

(event `StopLorenAnimation_0`
  ; Animation
  (goto _label_2 :!via `Stop`))

(event `ChangeTimeSpline_0`
  (params (NewTime :type "Float (single-precision)"))
  ; Animation
  (goto _label_2 :!via `SetNewTime`))

(event `self.ReceiveActorBeginOverlap`
  (params (OtherActor :type "Actor Object Reference"))
  (bind _spline (`/Game/Blueprints/Lore/BP_Spline.Spline` (`self.Spline_1`)))
  ; Animation
  (if (not (`self.InputBlock`))
    (`KismetSystemLibrary.Delay` 0.1)
    (if (`self.TotorialLore`)
      ;;[0.15 0.1304 0 0.5] LorenToto
      (`/Engine/EditorBlueprintResources/StandardMacros.IsValid` (`self.Spline_0`)
        (:`Is Valid`
          (`|ExecutionSequence`
            (:`then_0`
              (bind _pawninbox (`self.PushRayControl` (`self.BoxHinten`)))
              (if _pawninbox
                (`KismetSystemLibrary.PrintString` "pawn in box hinten")
                (if (not (`self.StopTotorialLoreVar`))
                  (goto _label))))
            (:`then_1`
              (bind _pawninbox_2 (`self.PushRayControl` (`self.BoxForne`)))
              (if _pawninbox_2
                (`KismetSystemLibrary.PrintString` "pawn in box Forne")
                (goto _label :!via `Reverse`))))))
      (else
        (`|ExecutionSequence`
          (:`then_0`
            (if (== (`self.LohreOnSplineCount`) 0)
              (`/Engine/EditorBlueprintResources/StandardMacros.IsValid` (`self.Spline_0`)
                (:`Is Valid`
                  (`|ExecutionSequence`
                    (:`then_0`
                      (bind _pawninbox_3 (`self.PushRayControl` (`self.BoxHinten`)))
                      (if _pawninbox_3
                        (`KismetSystemLibrary.PrintString` "pawn in box hinten")
                        (goto _label_2)))
                    (:`then_1`
                      (bind _pawninbox_4 (`self.PushRayControl` (`self.BoxForne`)))
                      (if _pawninbox_4
                        (`KismetSystemLibrary.PrintString` "pawn in box Forne")
                        (goto _label_2 :!via `Reverse`))))))))
          (:`then_1`
            (if (== (`self.LohreOnSplineCount`) 1)
              (`/Engine/EditorBlueprintResources/StandardMacros.IsValid` (`self.Spline_1`)
                (:`Is Valid`
                  (`|ExecutionSequence`
                    (:`then_0`
                      (bind _pawninbox_5 (`self.PushRayControl` (`self.BoxHinten`)))
                      (if _pawninbox_5
                        (bind (_direction _newtrack_0) (`Timeline|TimelineForSpline1` :`NewTime` (stale `ChangeTimeSpline_1` NewTime) :!label _label_3)
                          (:`Update`
                            (if (`self.Loren-Debug`)
                              (`KismetSystemLibrary.PrintString` (`KismetStringLibrary.Conv_DoubleToString` _newtrack_0) true true (struct :`R` 0.584079 :`G` 1.0 :`B` 0.14996 :`A` 0.501961) 5.0))
                            (bind _returnvalue (* _newtrack_0 (`SplineComponent.GetSplineLength` _spline)))
                            (`self.K2_SetActorLocationAndRotation` (`SplineComponent.GetLocationAtDistanceAlongSpline` _spline _returnvalue "World") (`SplineComponent.GetRotationAtDistanceAlongSpline` _spline _returnvalue "World"))))))
                    (:`then_1`
                      (bind _pawninbox_6 (`self.PushRayControl` (`self.BoxForne`)))
                      (if _pawninbox_6
                        (if (not (`self.StoneInFrontFromSpline1`))
                          (goto _label_3 :!via `Reverse`))))))))))))))

(event `BlockInput`
  (params (True :type Boolean))
  ; Animation
  ;; Aus Lohrenrotation
  (set `self.InputBlock` True))

(event `AktualisirungSpline1`
  ; Animation
  (goto _label_3))

(event `StopLorenAnimation_1`
  ; Animation
  (goto _label_3 :!via `Stop`))

(event `ChangeTimeSpline_1`
  (params (NewTime :type "Float (double-precision)"))
  ; Animation
  (goto _label_3 :!via `SetNewTime`))

(event `self.ReceiveBeginPlay`
  ;[0.15 0.08267 0 0.5] Debug
  (`|ExecutionSequence`
    (:`then_0`
      ; Aktualisirung
      (`KismetSystemLibrary.DelayUntilNextFrame`)
      (`self.ChangeTimeSpline_0` 0.0)
      (`self.AktualisirungSpline0` :!label _label_4)
      (`KismetSystemLibrary.DelayUntilNextTick`)
      (`self.StopLorenAnimation_0`))
    (:`then_1`
      (if (`KismetSystemLibrary.IsPackagedForDistribution`)
        (set `self.Loren-Debug` false)
        (elif (`self.Loren-Debug`)
          (`KismetSystemLibrary.PrintString` (`KismetStringLibrary.Concat_StrStr` "Loren-Debug in " (`KismetSystemLibrary.GetDisplayName` self) " is on") true true (struct :`R` 1.0 :`G` 0.361202 :`A` 0.504348) 7.0))))))

(event `Change spline`
  (params (spline :type Integer))
  ; Aktualisirung
  (bind _output_get (set `self.LohreOnSplineCount` spline))
  (switch `int` _output_get
    (:`0`
      (`self.ChangeTimeSpline_0` 3.86)
      (goto _label_4))
    (:`1`
      (`self.ChangeTimeSpline_1` 7.44)
      (`self.AktualisirungSpline1`)
      (`KismetSystemLibrary.DelayUntilNextTick`)
      (`self.StopLorenAnimation_1`))))

(fn `Interact`
  (params (Player :type "/Game/Blueprints/Player/BP_FirstPersionCharacter Object Reference"))
  (returns (PlayerInputBlock :type Boolean))
  (if (`self.TotorialLore`)
    (`/Game/Blueprints/BP_GitterTuer.interactWithLohre` (`self.Door`) Player)))

(fn `PushRayControl`
  (params (ToControllBox :type "BoxComponent Object Reference"))
  (returns (PawnInBox :type Boolean))
  (bind (_outactors _returnvalue) (`KismetSystemLibrary.BoxOverlapActors` (`SceneComponent.K2_GetComponentLocation` ToControllBox) (`BoxComponent.GetScaledBoxExtent` ToControllBox) (`|MakeArray` "ObjectTypeQuery3" :!type "EObjectTypeQuery Enum")))
  (if _returnvalue
    (for _array_element _outactors
      (`/Engine/EditorBlueprintResources/StandardMacros.IsValid` (`self.First Persion Character`)
        (:`Is Valid`
          (if (== (`self.First Persion Character`) _array_element)
            (return true)))
        (:`Is Not Valid`
          (bind _asbp_first_persion_character (cast `/Game/Blueprints/Player/BP_FirstPersionCharacter` _array_element))
          (set `self.First Persion Character` _asbp_first_persion_character)
          (return true))))
    (else
      (return false))))

(fn `UserConstructionScript`)