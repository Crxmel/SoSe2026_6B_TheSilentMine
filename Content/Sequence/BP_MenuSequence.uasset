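; BP_MenuSequence plays the MenuSequence level sequence as a looping backdrop until the player presses play.
; On BeginPlay it starts the endless loop, waits one frame, then finds BP_FirstPersionCharacter and binds to the PressPlay dispatcher on its MainUI.
; When that event fires, the sequence player stops.
; A leftover "Hello" print is unconnected and never runs.
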(event `self.ReceiveBeginPlay`
  (`MovieSceneSequencePlayer.PlayLooping` (`LevelSequenceActor.SequencePlayer` (`self.MenuSequence`)) -1)
  (`KismetSystemLibrary.DelayUntilNextFrame`)
  (bind _returnvalue (`GameplayStatics.GetActorOfClass` "/Game/Blueprints/Player/BP_FirstPersionCharacter.BP_FirstPersionCharacter_C"))
  (add `/Game/Blueprints/UI/BPW_MainUI.PressPlay` (`/Game/Blueprints/Player/BP_FirstPersionCharacter.MainUI` _returnvalue) (delegate `PressPlay_Event`)))

(event `PressPlay_Event`
  (`MovieSceneSequencePlayer.Stop` (`LevelSequenceActor.SequencePlayer` (`self.MenuSequence`))))

(fn `UserConstructionScript`)