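; BP_Sequence directs the game's cinematics, from the looping menu sequence through the start cutscene to the end sequence.
; It waits for the player character, binds its Play button, and uses Debug to skip the menu and unlock input in non-distribution builds.
; A timeline drives a post-process fade material, with FadeNumber selecting the follow-up sequence or level restart.
; Cutscene events swap breakable boards, animate a falling board and play camera-located sounds.
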(event `self.ReceiveBeginPlay`
  (bind _player (`self.Player`))
  (bind _mainui (`/Game/Blueprints/Player/BP_FirstPersionCharacter.MainUI` _player))
  (`SceneComponent.SetVisibility` (`StaticMeshActor.StaticMeshComponent` (`self.EndAnimationFallingBoard`)) false false)
  (`|ExecutionSequence`
    (:`then_0`
      ; Debug
      (if (`KismetSystemLibrary.IsPackagedForDistribution`)
        (set `self.Debug` false)))
    (:`then_1`
      ; notWalkBlock wenn sequenser off/ debug on
      (`|ExecutionSequence`
        (:`then_0`
          ; Post Process Material für fade in / out
          (bind _returnvalue (`KismetMaterialLibrary.CreateDynamicMaterialInstance` "/Game/Sequence/MM_PP_Fade.MM_PP_Fade"))
          (bind _output_get (set `self.PostProcessMaterial` _returnvalue))
          (setmembers `PostProcessSettings` :`StructRef` (`PostProcessVolume.Settings` (`self.PostProsses`)) :`WeightedBlendables` (make `WeightedBlendables` (`|MakeArray` (make `WeightedBlendable` 1.0 _output_get) (make `WeightedBlendable` 1.0 "/Game/Material/PPV_Fog_Inst.PPV_Fog_Inst"))))
          (if (not (`self.Debug`))
            (`MovieSceneSequencePlayer.PlayLooping` (`LevelSequenceActor.SequencePlayer` (`self.MenuSequence`)) -1))
          (`KismetSystemLibrary.DelayUntilNextFrame`)
          (bind _returnvalue_2 (`GameplayStatics.GetActorOfClass` "/Game/Blueprints/Player/BP_FirstPersionCharacter.BP_FirstPersionCharacter_C" :!label _label))
          (bind _output_get_2 (set `self.Player` _returnvalue_2))
          (`/Engine/EditorBlueprintResources/StandardMacros.IsValid` _output_get_2
            (:`Is Valid`
              (bind _mainui_2 (`/Game/Blueprints/Player/BP_FirstPersionCharacter.MainUI` _output_get_2))
              (add `/Game/Blueprints/UI/BPW_MainUI.PressPlayFirstTime` _mainui_2 (delegate `PressPlay_Event`))
              (if (`self.Debug`)
                (`Widget.SetVisibility` (`/Game/Blueprints/UI/BPW_MainUI.StartOverlay` _mainui_2) "Hidden")
                (set `PlayerController.bShowMouseCursor` false (`GameplayStatics.GetPlayerController` 0))))
            (:`Is Not Valid`
              (`KismetSystemLibrary.DelayUntilNextTick`)
              (goto _label))))
        (:`then_1`
          (if (`self.Debug`) :!label _label_2
            (`/Engine/EditorBlueprintResources/StandardMacros.IsValid` _player
              (:`Is Valid`
                (set `/Game/Blueprints/Player/BP_FirstPersionCharacter.InputBlock` false _player)
                (`SceneComponent.SetVisibility` (`/Game/Blueprints/Player/BP_FirstPersionCharacter.SpotLight` _player) true false)
                (`SceneComponent.SetVisibility` (`/Game/Blueprints/Player/BP_FirstPersionCharacter.PointLight` _player) true false)
                (set `/Game/Blueprints/UI/BPW_MainUI.UI IsOpen` false _mainui)
                (set `/Game/Blueprints/UI/BPW_MainUI.PausedIsBlock` false _mainui)
                (`/Game/Blueprints/UI/BPW_MainUI.ChangeMousCursor` _mainui))
              (:`Is Not Valid`
                (`KismetSystemLibrary.DelayUntilNextFrame`)
                (goto _label_2)))))))))

(event `PressPlay_Event`
  ; PresPlayButton
  (`self.PlayFade` true 1))

(event `FadeEnd_0`
  ; PresPlayButton
  (`MovieSceneSequencePlayer.Stop` (`LevelSequenceActor.SequencePlayer` (`self.MenuSequence`)))
  (`MovieSceneSequencePlayer.Play` (`LevelSequenceActor.SequencePlayer` (`self.StartSequencer`)))
  (`self.PlayFade` false))

(event `BreakBretter`
  ; Aus cutscreen
  (`SceneComponent.SetVisibility` (`StaticMeshActor.StaticMeshComponent` (`self.EinzubechendeBrettgroup`)) false false)
  (`SceneComponent.SetVisibility` (`Actor.RootComponent` (`self.EinzubechendeBrettgroup_Kaputt`)) true false))

(event `PlayFade`
  (params (`Fade in` :type Boolean) (FadeNumber :type Integer))
  ; Fade
  (if `Fade in`
    (bind (_direction _fadefload) (`Timeline|Fade out` :!via `PlayFromStart` :!label _label_3)
      (:`Update`
        (`MaterialInstanceDynamic.SetScalarParameterValue` (`self.PostProcessMaterial`) "Alpha" _fadefload))
      (:`Finished`
        (switch `int` FadeNumber
          (:`1`
            (`self.FadeEnd_0`))
          (:`2`
            (`|ExecutionSequence`
              (:`then_0`
                (`/Engine/EditorBlueprintResources/StandardMacros.DoOnce` false
                  (:`Completed`
                    (`self.SequenceEvent_PlayEndSequence` true)
                    (goto _label_4 :!via `Reset`))))
              (:`then_1`
                (`/Engine/EditorBlueprintResources/StandardMacros.DoOnce` true :!label _label_4
                  (:`Completed`
                    (`self.SequenceEvent_PlayEndSequence` true true))))))
          (:`3`
            (`KismetSystemLibrary.ExecuteConsoleCommand` "RestartLevel" null))
          (:`4`
            ;; Ende from Start Scene
            (`KismetSystemLibrary.Delay` 1.0)
            (`self.PlayFade` false 5))
          (:`5`
            (`KismetSystemLibrary.Delay` 0.5)
            (`self.SequenceEvent_OlayEndFromStartScreen-`)))))
    (else
      (goto _label_3 :!via `ReverseFromEnd`))))

(event `SequenceEvent_PlayEndSequence`
  (params (FadeIn_hasPlay :type Boolean) (FAdeOut_hasPlay :type Boolean))
  ; Play EndSequence
  (if FadeIn_hasPlay
    (if FAdeOut_hasPlay
      (`MovieSceneSequencePlayer.Play` (`LevelSequenceActor.SequencePlayer` (`self.EndSequence`)))
      (set `/Game/Blueprints/Player/BP_FirstPersionCharacter.InputBlock` true (`self.Player`))
      (`SceneComponent.SetVisibility` (`/Game/Blueprints/Player/BP_FirstPersionCharacter.SpotLight` (`self.Player`)) false false)
      (else
        (`self.PlayFade` false 2)))
    (else
      (`self.PlayFade` true 2))))

(event `Endsequence_FallingBoard_Visibillty`
  ; Play EndSequence
  (`SceneComponent.SetVisibility` (`StaticMeshActor.StaticMeshComponent` (`self.EndAnimationFallingBoard`)) true false))

(event `EndSequence_FallingBoard_Animation`
  (bind (_returnvalue_roll _returnvalue_pitch _returnvalue_yaw) (`KismetMathLibrary.BreakRotator` (`SceneComponent.K2_GetComponentRotation` (`StaticMeshActor.StaticMeshComponent` (`self.EndAnimationFallingBoard`)))))
  ; Play EndSequence
  (set `self.EndAnimationFallingBoard_WorlRotationY` _returnvalue_pitch)
  (bind (_direction _newtrack_0) (`Timeline|EndSceneFallingBoardAnimation` :!via `PlayFromStart`)
    (:`Update`
      (`SceneComponent.K2_SetWorldRotation` (`StaticMeshActor.StaticMeshComponent` (`self.EndAnimationFallingBoard`)) (`KismetMathLibrary.MakeRotator` _returnvalue_roll (* _newtrack_0 (`self.EndAnimationFallingBoard_WorlRotationY`)) _returnvalue_yaw) false false))))

(fn `PlaySoundOnCamera`
  (params (CameraComponent :type "CameraComponent Object Reference") (Sound :type "SoundBase Object Reference"))
  (`/Engine/EditorBlueprintResources/StandardMacros.IsValid` CameraComponent
    (:`Is Valid`
      (`GameplayStatics.PlaySoundAtLocation` Sound (`SceneComponent.K2_GetComponentLocation` (`local.CameraComponent`)) (struct) 1.0 1.0 0.0 null null null null))
    (:`Is Not Valid`
      (`KismetSystemLibrary.PrintString` "BP_sequencer dont has cam component"))))

(fn `UserConstructionScript`)